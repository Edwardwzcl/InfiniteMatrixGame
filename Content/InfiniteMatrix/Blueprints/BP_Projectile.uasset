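; BP_Projectile is a short-lived projectile that awards the player score when it hits an enemy.
; On BeginPlay it caches the player pawn as BP_Player and sets a lifespan so it expires on its own.
; Overlapping a BP_Enemy increments the player's Score, refreshes the score UI and destroys the projectile, while overlapping a BP_Tunnel only destroys it.
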(event EventBeginPlay
  (bind _asbp_player (Utilities|Casting|CastToBP_Player (Game|Player|GetPlayerPawn 0)))
  (Variables|Default|SetPlayerRef _asbp_player)
  (Actor|SetLifeSpan 3.0))

(event Collision|EventActorBeginOverlap
  (params (OtherActor :type Actor%20Object%20Reference))
  (bind _playerref (Variables|Default|GetPlayerRef))
  (Utilities|Casting|CastToBP_Enemy OtherActor
    (:then
      (bind _output_get (Variables|/Game/InfiniteMatrix/Blueprints/BP_Player.BP_Player_C|SetScore _playerref (+ (Variables|/Game/InfiniteMatrix/Blueprints/BP_Player.BP_Player_C|GetScore _playerref) 1)))
      (Default|UpdateScoreUI (Variables|/Game/InfiniteMatrix/Blueprints/BP_Player.BP_Player_C|GetScoreUIRef _playerref) _output_get)
      (Actor|DestroyActor))
    (:CastFailed
      (Utilities|Casting|CastToBP_Tunnel OtherActor)
      (Actor|DestroyActor))))

(event EventTick
  (params (DeltaSeconds :type Float%20%28single-precision%29)))

(fn ConstructionScript)