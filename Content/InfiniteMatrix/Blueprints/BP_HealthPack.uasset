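; Health pack pickup Blueprint that heals the player on contact and expires if left uncollected.
; On BeginPlay it caches the player pawn as BP_Player and sets a short lifespan, which is skipped if the cast fails.
; When that player overlaps the trigger, it adds HealAmount to Health clamped to MaxHealth, refreshes the health bar widget directly and destroys itself.
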(event OnComponentBeginOverlap(HealthPackTrigger)
  (params (OverlappedComponent :type Primitive%20Component%20Object%20Reference) (OtherActor :type Actor%20Object%20Reference) (OtherComp :type Primitive%20Component%20Object%20Reference) (OtherBodyIndex :type Integer) (bFromSweep :type Boolean) (SweepResult :type Hit%20Result%20Structure%20%28by%20ref%29))
  (bind _bp_playerref (Variables|Default|GetBP_PlayerRef))
  (if (== OtherActor (Variables|Default|GetBP_PlayerRef))
    (bind _output_get (Variables|/Game/InfiniteMatrix/Blueprints/BP_Player.BP_Player_C|SetHealth _bp_playerref (Math|Float|Clamp(Float) (+ (Variables|/Game/InfiniteMatrix/Blueprints/BP_Player.BP_Player_C|GetHealth _bp_playerref) (Variables|Default|GetHealAmount)) 0.0 (Variables|/Game/InfiniteMatrix/Blueprints/BP_Player.BP_Player_C|GetMaxHealth _bp_playerref))))
    (Default|UpdateHealthUI (Variables|/Game/InfiniteMatrix/Blueprints/BP_Player.BP_Player_C|GetHealthBarRef _bp_playerref) _output_get (Variables|/Game/InfiniteMatrix/Blueprints/BP_Player.BP_Player_C|GetMaxHealth _bp_playerref))
    (Actor|DestroyActor)))

(event EventBeginPlay
  (bind _asbp_player (Utilities|Casting|CastToBP_Player (Game|Player|GetPlayerPawn 0)))
  (Variables|Default|SetBP_PlayerRef _asbp_player)
  (Actor|SetLifeSpan 1e+01))

(fn ConstructionScript)